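; Click-to-move player character for a 2D prototype, flipping to face its horizontal travel direction.
; A left click stores the deprojected mouse position, with floored X and Y and the capsule's Z, as the target, without any trace.
; Tick reissues Simple Move To Location toward that target and sets rotation from X velocity, with a small dead zone below zero.
; Tick also prints a leftover debug string every frame.
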(event EventBeginPlay
  (Variables|Default|SetTargetPlayerLocation (Transformation|GetWorldLocation (Variables|Collision|GetCapsuleComponent))))

(event EventTick
  (params (DeltaSeconds :type Float%20%28single-precision%29))
  (bind _returnvalue (Transformation|GetVelocity))
  (AI|Navigation|SimpleMovetoLocation (Game|GetPlayerController 0) (Variables|Default|GetTargetPlayerLocation))
  (Development|PrintString "Azi nike ta mère")
  (if (>= (.x _returnvalue) 0.0) ; Change son orientation en fonction de ses déplacement
    (Transformation|SetActorRotation "0.000000,0.000000,0.000000")
    (elif (< (.x _returnvalue) -1.0)
      (Transformation|SetActorRotation "-180.000000,0.000000,0.000000"))))

(event Input|MouseEvents|LeftMouseButton
  (params (Key :type Key%20Structure :default "None"))
  (bind _returnvalue (Game|GetPlayerController 0))
  (bind _worldlocation (Game|Player|ConvertMouseLocationToWorldSpace _returnvalue))
  ;[0 0 0] Déplace le player e l'endroit cliqué
  (:Pressed
    (Variables|Default|SetTargetPlayerLocation (Math|Vector|MakeVector (Math|Conversions|ToFloat(Integer) (Math|Float|Floor (.x _worldlocation))) (Math|Conversions|ToFloat(Integer) (Math|Float|Floor (.y _worldlocation))) (.z (Transformation|GetWorldLocation (Variables|Collision|GetCapsuleComponent)))))))

(fn ConstructionScript)