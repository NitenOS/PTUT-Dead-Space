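; BP_Fouille is a searchable spot ("fouille") that gives BP_Char2D5 an item a single time.
; Box begin overlap stores the character, sets its IsTriggerFouille flag and registers itself as FouilleBP.
; The Fouille event uses DoOnce to add Image to the character's Item array and Name to Inventary.
; End overlap also sets IsTriggerFouille to true, so leaving the box never clears it.
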(event OnComponentBeginOverlap(Box)
  (params (OverlappedComponent :type Primitive%20Component%20Object%20Reference) (OtherActor :type Actor%20Object%20Reference) (OtherComp :type Primitive%20Component%20Object%20Reference) (OtherBodyIndex :type Integer) (bFromSweep :type Boolean) (SweepResult :type Hit%20Result%20Structure%20%28by%20ref%29))
  (bind _asbp_char_2d5 (Utilities|Casting|CastToBP_Char2D5 OtherActor))
  (Variables|/Game/Proto2D5/Bleuprint/BP_Char2D5.BP_Char2D5_C|SetIsTriggerFouille _asbp_char_2d5 true)
  (Variables|Default|SetAs%20BP%20Char%202D5 _asbp_char_2d5)
  (Variables|/Game/Proto2D5/Bleuprint/BP_Char2D5.BP_Char2D5_C|SetFouilleBP _asbp_char_2d5 self))

(event OnComponentEndOverlap(Box)
  (params (OverlappedComponent :type Primitive%20Component%20Object%20Reference) (OtherActor :type Actor%20Object%20Reference) (OtherComp :type Primitive%20Component%20Object%20Reference) (OtherBodyIndex :type Integer))
  (bind _asbp_char_2d5 (Utilities|Casting|CastToBP_Char2D5 OtherActor))
  (Variables|/Game/Proto2D5/Bleuprint/BP_Char2D5.BP_Char2D5_C|SetIsTriggerFouille _asbp_char_2d5 true))

(event Custom|Fouille
  (bind _as_bp_char_2d5 (Variables|Default|GetAs%20BP%20Char%202D5))
  (Utilities|FlowControl|DoOnce false
    (:Completed
      (Utilities|Array|Add (Variables|/Game/Proto2D5/Bleuprint/BP_Char2D5.BP_Char2D5_C|GetItem _as_bp_char_2d5) (Variables|Default|GetImage))
      (Utilities|Array|Add (Variables|/Game/Proto2D5/Bleuprint/BP_Char2D5.BP_Char2D5_C|GetInventary _as_bp_char_2d5) (Variables|Default|GetName)))))

(event EventBeginPlay)

(event Collision|EventActorBeginOverlap
  (params (OtherActor :type Actor%20Object%20Reference)))

(event EventTick
  (params (DeltaSeconds :type Float%20%28single-precision%29)))

(fn ConstructionScript)