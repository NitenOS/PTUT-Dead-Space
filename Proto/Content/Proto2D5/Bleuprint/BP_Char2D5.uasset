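; Player worker character for a 2.5D Paper2D prototype: walks with flipbook animation, calls Isaac over, searches spots and collects items into an inventory widget.
; F toggles an Isaac customization mode that swaps Isaac for spawned bust and arm part actors, blends the camera, then applies the chosen arm sprites on exit.
; In that mode, the mouse grabs "CanBeGrab" components, which Tick drags along the deprojected cursor, locked to Isaac's depth.
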(event OnComponentBeginOverlap(CapsuleComponent)
  (params (OverlappedComponent :type Primitive%20Component%20Object%20Reference) (OtherActor :type Actor%20Object%20Reference) (OtherComp :type Primitive%20Component%20Object%20Reference) (OtherBodyIndex :type Integer) (bFromSweep :type Boolean) (SweepResult :type Hit%20Result%20Structure%20%28by%20ref%29))
  ;[0 0 0] Set des objet
  (bind _asbp_caisse (Utilities|Casting|CastToBP_Caisse OtherActor))
  (Variables|Default|SetCaisseBP _asbp_caisse))

(event EventTick
  (params (DeltaSeconds :type Float%20%28single-precision%29))
  (bind _returnvalue (Game|GetPlayerController 0))
  (bind _distancegrabobjet (Variables|Default|GetDistanceGrabObjet))
  (bind (_worldlocation _worlddirection) (Game|Player|ConvertMouseLocationToWorldSpace _returnvalue))
  (bind _returnvalue_2 (* _worlddirection _distancegrabobjet))
  (bind _returnvalue_3 (+ _worldlocation _returnvalue_2))
  ;[1 1 1] Update
  (if (Variables|Default|GetIsGrabing)
    (Transformation|SetWorldLocation (Variables|Default|GetHit%20Component) (Math|Vector|MakeVector (.x _returnvalue_3) (.y (Variables|Default|GetIsaacWorldLocation)) (.z _returnvalue_3)) false false)))

(event EventBeginPlay
  ;[0 0 0] Add inventary Widget
  (bind _returnvalue (UserInterface|CreateWidget "/Game/Proto2D5/Interface/WBP_Inventary.WBP_Inventary_C"))
  (bind _output_get (Variables|Default|SetInventory _returnvalue))
  (bind _returnvalue_2 (UserInterface|CreateWidget "/Game/Proto2D5/Interface/WBP_Key.WBP_Key_C"))
  (UserInterface|Viewport|AddtoViewport _output_get 0))

(event Input|AxisEvents|InputAxisForward2D5
  (params (AxisValue :type Float%20%28single-precision%29))
  (bind _sprite (Variables|Default|GetSprite))
  ;[0 0 0] Move left/right
  (if (not (Variables|Default|GetInteractingIsaac))
    (Utilities|FlowControl|Sequence
      (:then_0
        (Pawn|Input|AddMovementInput "1.000000,0.000000,0.000000" AxisValue false)
        (if (== AxisValue -2.0)
          (Transformation|SetWorldRotation (Variables|Default|GetSprite) "0.000000,-180.000000,-0.000000" false false)
          (elif (== AxisValue 2.0)
            (Transformation|SetWorldRotation (Variables|Default|GetSprite) "0, 0, 0" false false))))
      (:then_1
        (if (== AxisValue 0.0)
          (Sprite|SetFlipbook _sprite "/Game/Proto2D5/Test_Tori/Fixed_Sprite/Ouvrier/FB_Idle_Ouvrier_Redim.FB_Idle_Ouvrier_Redim")
          (else
            (Sprite|SetFlipbook _sprite "/Game/Proto2D5/Test_Tori/Fixed_Sprite/Ouvrier/FB_Ouvrier.FB_Ouvrier")))))))

(event Input|AxisEvents|InputAxisBack2D5
  (params (AxisValue :type Float%20%28single-precision%29))
  ;[0 0 0] Move forward/back
  (Utilities|FlowControl|Sequence
    (:then_0
      (if (not (Variables|Default|GetInteractingIsaac))
        (Pawn|Input|AddMovementInput "0.000000,1.000000,0.000000" AxisValue false)))
    (:then_1
      (if (not (== AxisValue 0.0))
        (Sprite|SetFlipbook (Variables|Default|GetSprite) "/Game/Proto2D5/Test_Tori/Fixed_Sprite/Ouvrier/FB_Ouvrier.FB_Ouvrier")))))

(event Input|KeyboardEvents|E
  (params (Key :type Key%20Structure :default "None"))
  (bind _objectbp (Variables|Default|GetObjectBP))
  (bind _objectbp_2 (Variables|Default|GetObjectBP))
  ;[0 0 0] Interact "E" (with "BP_Fouille" et BP_Object")
  (:Pressed
    (if (Variables|Default|GetIsTriggerFouille)
      (Default|FOUILLE (Variables|Default|GetFouilleBP))
      (elif (and (Variables|/Game/Proto2D5/Bleuprint/BP_Object.BP_Object_C|GetCanBeDestroyed _objectbp) (Variables|/Game/Proto2D5/Bleuprint/BP_Object.BP_Object_C|GetIsInItemBox _objectbp))
        (if (Variables|Default|GetFirstItem)
          (Variables|Default|SetFirstItem false)
          (else
            (Class|PanelWidget|RemoveChildat (Variables|/Game/Proto2D5/Interface/WBP_Inventary.WBP_Inventary_C|GetVerticalBox_79 (Variables|Default|GetInventory)))))
        (bind _returnvalue (UserInterface|CreateWidget "/Game/Proto2D5/Interface/WBP_Item.WBP_Item_C" 0 (Utilities|Text|ToText(String) (Variables|/Game/Proto2D5/Bleuprint/BP_Object.BP_Object_C|GetItemName _objectbp_2)) (Variables|/Game/Proto2D5/Bleuprint/BP_Object.BP_Object_C|GetSpriteInventary _objectbp_2)))
        (Class|VerticalBox|AddChildtoVerticalBox (Variables|/Game/Proto2D5/Interface/WBP_Inventary.WBP_Inventary_C|GetVerticalBox_79 (Variables|Default|GetInventory)) _returnvalue)
        (Default|AddItem (Variables|Default|GetObjectBP))))))

(event Input|KeyboardEvents|F
  (params (Key :type Key%20Structure :default "None"))
  (bind _isaacbp (Variables|Default|GetIsaacBP))
  (:Pressed
    (if (or (Variables|Default|GetIsInteractableIsaac) (Variables|Default|GetInteractingIsaac))
      (Utilities|ShowCursor
        (:Out
          (if (Variables|Default|GetInteractingIsaac)
            (Default|Reaparition (Variables|Default|GetIsaacBP))
            (Rendering|Components|Sprite|SetSprite (Variables|/Game/Proto2D5/Bleuprint/BP_Isaac1.BP_Isaac1_C|GetBras%20Gauche (Variables|Default|GetIsaacBP)) (Variables|/Game/Proto2D5/Bleuprint/BP_IsaacPart/BP_PartBusteTete.BP_PartBusteTete_C|GetBrasGSPR (Variables|Default|GetNewBuste)))
            (Rendering|Components|Sprite|SetSprite (Variables|/Game/Proto2D5/Bleuprint/BP_Isaac1.BP_Isaac1_C|GetBras%20Droit (Variables|Default|GetIsaacBP)) (Variables|/Game/Proto2D5/Bleuprint/BP_IsaacPart/BP_PartBusteTete.BP_PartBusteTete_C|GetBrasDSPR (Variables|Default|GetNewBuste)))
            (Default|DesTruite (Variables|Default|GetNewBrasG))
            (Default|DesTruite (Variables|Default|GetNewBrasD))
            (Game|Player|SetViewTargetwithBlend (Game|GetPlayerController 0) self 1.0 "VTBlend_Linear" 0.0 false)
            (Utilities|FlowControl|Delay 1.0)
            (Default|DesTruite (Variables|Default|GetNewBuste))
            (if (Variables|Default|GetFirstItem)
              _
              (else
                (Actor|DestroyActor (Variables|Default|GetTempObject))))
            (Variables|Default|SetInteractingIsaac false)
            (else
              (Variables|Default|SetIsaacWorldLocation (Transformation|GetWorldLocation (Variables|/Script/Engine.Character|GetCapsuleComponent (Variables|Default|GetIsaacBP))))
              (Variables|Default|SetArmMoveBox false)
              (Variables|Default|SetInteractingIsaac true)
              (Utilities|PlacementDeL'ouvrier
                (:Out
                  (bind _returnvalue (Game|SpawnActorfromClass (Variables|Inventaire|GetUniqueItemFull) (Math|Conversions|ToTransform(Vector) (+ (Variables|Default|GetIsaacWorldLocation) (Math|Vector|MakeVector -1.5e+02 0.0 0.0))) "Undefined" "MultiplyWithRoot" 0 0))
                  (Variables|Default|SetTempObject _returnvalue)
                  (bind _returnvalue_2 (Game|SpawnActorfromClass "/Game/Proto2D5/Bleuprint/BP_IsaacPart/BP_PartBrasG.BP_PartBrasG_C" (Math|Conversions|ToTransform(Vector) (Transformation|GetWorldLocation (Variables|/Game/Proto2D5/Bleuprint/BP_Isaac1.BP_Isaac1_C|GetBras%20Gauche _isaacbp))) "Undefined" "MultiplyWithRoot" 0 0))
                  (bind _output_get (Variables|Default|SetNewBrasG _returnvalue_2))
                  (Rendering|Components|Sprite|SetSprite (Variables|/Game/Proto2D5/Bleuprint/BP_IsaacPart/BP_PartBrasG.BP_PartBrasG_C|GetSprite _output_get) (Sprite|GetSprite (Variables|/Game/Proto2D5/Bleuprint/BP_Isaac1.BP_Isaac1_C|GetBras%20Gauche _isaacbp)))
                  (bind _returnvalue_3 (Game|SpawnActorfromClass "/Game/Proto2D5/Bleuprint/BP_IsaacPart/BP_PartBrasD.BP_PartBrasD_C" (Math|Conversions|ToTransform(Vector) (Transformation|GetWorldLocation (Variables|/Game/Proto2D5/Bleuprint/BP_Isaac1.BP_Isaac1_C|GetBras%20Droit _isaacbp))) "Undefined" "MultiplyWithRoot" 0 0))
                  (bind _output_get_2 (Variables|Default|SetNewBrasD _returnvalue_3))
                  (Rendering|Components|Sprite|SetSprite (Variables|/Game/Proto2D5/Bleuprint/BP_IsaacPart/BP_PartBrasD.BP_PartBrasD_C|GetSprite _output_get_2) (Sprite|GetSprite (Variables|/Game/Proto2D5/Bleuprint/BP_Isaac1.BP_Isaac1_C|GetBras%20Droit _isaacbp)))
                  (bind _returnvalue_4 (Game|SpawnActorfromClass "/Game/Proto2D5/Bleuprint/BP_IsaacPart/BP_PartBusteTete.BP_PartBusteTete_C" (Math|Conversions|ToTransform(Vector) (Transformation|GetWorldLocation (Variables|/Game/Proto2D5/Bleuprint/BP_Isaac1.BP_Isaac1_C|GetBuste _isaacbp))) "Undefined" "MultiplyWithRoot" 0 0))
                  (bind _output_get_3 (Variables|Default|SetNewBuste _returnvalue_4))
                  (Game|Player|SetViewTargetwithBlend (Game|GetPlayerController 0) _output_get_3 1.0 "VTBlend_Linear" 0.0 false)
                  (Default|Disparition (Variables|Default|GetIsaacBP)))))))))))

(event Input|MouseEvents|LeftMouseButton
  (params (Key :type Key%20Structure :default "None"))
  ;[0 0 0] Grip
  (:Pressed
    (if (Variables|Default|GetInteractingIsaac)
      (Utilities|GrabComponent
        (:Out
          (Variables|Default|SetIsGrabing true)))))
  (:Released
    (if (Variables|Default|GetInteractingIsaac)
      (Variables|Default|SetHit%20Component 0)
      (Physics|Components|PhysicsHandle|ReleaseComponent (Variables|Default|GetPhysicsHandle))
      (Variables|Default|SetIsGrabing false))))

(event Input|KeyboardEvents|A
  (params (Key :type Key%20Structure :default "None"))
  ;[0 0 0] Move Isaac
  (:Pressed
    (Default|MoveToo (Variables|Default|GetIsaacBP) (Transformation|GetActorLocation))))

(event Input|KeyboardEvents|SpaceBar
  (params (Key :type Key%20Structure :default "None"))
  ;[0 0 0] Move caisse
)

(fn ConstructionScript)