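; BP_Caisse is a crate that BP_Isaac1 can push when the right arm shows the piston sprite.
; Overlapping its Box with that sprite sets CanMoveBox on Isaac and the crate's CanDo flag; leaving clears only CanMoveBox.
; The Move event teleports the Cube a fixed step along Y without sweep while CanDo is set.
; Debug prints report the move and the Cube's location every tick.
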(event OnComponentBeginOverlap(Box)
  (params (OverlappedComponent :type Primitive%20Component%20Object%20Reference) (OtherActor :type Actor%20Object%20Reference) (OtherComp :type Primitive%20Component%20Object%20Reference) (OtherBodyIndex :type Integer) (bFromSweep :type Boolean) (SweepResult :type Hit%20Result%20Structure%20%28by%20ref%29))
  (bind _asbp_isaac_1 (Utilities|Casting|CastToBP_Isaac1 OtherActor))
  (if (== (Sprite|GetSprite (Variables|/Game/Proto2D5/Bleuprint/BP_Isaac1.BP_Isaac1_C|GetBras%20Droit _asbp_isaac_1)) "/Game/Proto2D5/Test_Tori/Fixed_Sprite/Isaac/Membres_Droit/D_Bras_piston_v2_Redim_Sprite.D_Bras_piston_v2_Redim_Sprite")
    (bind _output_get (Variables|/Game/Proto2D5/Bleuprint/BP_Isaac1.BP_Isaac1_C|SetCanMoveBox _asbp_isaac_1 true))
    (Variables|Default|SetCanDo _output_get)))

(event OnComponentEndOverlap(Box)
  (params (OverlappedComponent :type Primitive%20Component%20Object%20Reference) (OtherActor :type Actor%20Object%20Reference) (OtherComp :type Primitive%20Component%20Object%20Reference) (OtherBodyIndex :type Integer))
  (bind _asbp_isaac_1 (Utilities|Casting|CastToBP_Isaac1 OtherActor))
  (bind _output_get (Variables|/Game/Proto2D5/Bleuprint/BP_Isaac1.BP_Isaac1_C|SetCanMoveBox _asbp_isaac_1 false)))

(event Custom|Move
  (if (Variables|Default|GetCanDo)
    (Development|PrintString "enter")
    (Transformation|SetWorldLocation (Variables|Default|GetCube) (+ (Transformation|GetWorldLocation (Variables|Default|GetCube)) "0.000000,400.000000,0.000000") false false)))

(event EventTick
  (params (DeltaSeconds :type Float%20%28single-precision%29))
  (Development|PrintString (Utilities|String|ToString(Vector) (Transformation|GetWorldLocation (Variables|Default|GetCube)))))

(fn ConstructionScript)