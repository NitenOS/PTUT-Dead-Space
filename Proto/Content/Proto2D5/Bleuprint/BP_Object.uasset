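; BP_Object is a pickup item that BP_Char2D5 collects by touching its Box collision.
; A delay on BeginPlay keeps it from being picked up for the first two seconds after spawn, through the CanBeDestroyed flag.
; A valid overlap writes its name and two sprites into the character's single inventory slot, without checking what it holds, then destroys the actor.
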(event OnComponentBeginOverlap(Box)
  (params (OverlappedComponent :type Primitive%20Component%20Object%20Reference) (OtherActor :type Actor%20Object%20Reference) (OtherComp :type Primitive%20Component%20Object%20Reference) (OtherBodyIndex :type Integer) (bFromSweep :type Boolean) (SweepResult :type Hit%20Result%20Structure%20%28by%20ref%29))
  ;[0 0 0] Add Item
  (bind _asbp_char_2d5 (Utilities|Casting|CastToBP_Char2D5 OtherActor))
  (if (Variables|Default|GetCanBeDestroyed)
    (bind _output_get (Variables|Default|SetChar2D5BP _asbp_char_2d5))
    (Variables|/Game/Proto2D5/Bleuprint/BP_Char2D5.BP_Char2D5_C|SetUniqueInventary _output_get (Variables|Default|GetItemName))
    (Variables|/Game/Proto2D5/Bleuprint/BP_Char2D5.BP_Char2D5_C|SetUniqueItemFull (Variables|Default|GetChar2D5BP) (Variables|Default|GetSpriteFull))
    (Variables|/Game/Proto2D5/Bleuprint/BP_Char2D5.BP_Char2D5_C|SetUniqueItemInventary (Variables|Default|GetChar2D5BP) (Variables|Default|GetSpriteInventary))
    (Actor|DestroyActor)))

(event EventBeginPlay
  ;[1 0 0] A voir avec le prof comment on peut le rendre rmassable qu'après 2s suivant le spawn
  (Variables|Default|SetCanBeDestroyed false)
  (Utilities|FlowControl|Delay 2.0)
  (Variables|Default|SetCanBeDestroyed true))

(fn ConstructionScript)