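; BP_Isaac is an interactable character in the 2.5D prototype, built from separate body-part components.
; Overlapping its BigBox sets an interaction flag and self-reference on BP_Char2D5; leaving clears only the flag.
; Two events await outside callers: MoveToo walks it to a given location via AIMoveTo, and Disparition destroys it.
; Destruction also fires the end overlap, closing interaction; the debug-print and visibility-toggle nodes are unconnected.
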(event OnComponentBeginOverlap(BigBox)
  (params (OverlappedComponent :type Primitive%20Component%20Object%20Reference) (OtherActor :type Actor%20Object%20Reference) (OtherComp :type Primitive%20Component%20Object%20Reference) (OtherBodyIndex :type Integer) (bFromSweep :type Boolean) (SweepResult :type Hit%20Result%20Structure%20%28by%20ref%29))
  (bind _asbp_char_2d5 (Utilities|Casting|CastToBP_Char2D5 OtherActor))
  (Variables|/Game/Proto2D5/Bleuprint/BP_Char2D5.BP_Char2D5_C|SetIsInteractableIsaac _asbp_char_2d5 true)
  (Variables|/Game/Proto2D5/Bleuprint/BP_Char2D5.BP_Char2D5_C|SetIsaacBP _asbp_char_2d5 self))

(event OnComponentEndOverlap(BigBox)
  (params (OverlappedComponent :type Primitive%20Component%20Object%20Reference) (OtherActor :type Actor%20Object%20Reference) (OtherComp :type Primitive%20Component%20Object%20Reference) (OtherBodyIndex :type Integer))
  ;[1 0 0] Ca ça s'active quand le truc est détruit donc plus d'interaction possible
  (bind _asbp_char_2d5 (Utilities|Casting|CastToBP_Char2D5 OtherActor))
  (Variables|/Game/Proto2D5/Bleuprint/BP_Char2D5.BP_Char2D5_C|SetIsInteractableIsaac _asbp_char_2d5 false))

(event Custom|Disparition
  (Actor|DestroyActor))

(event Custom|MoveToo
  (params (PlayerLocation :type Vector))
  (AI|AIMoveTo self PlayerLocation 0 1e+02 false))

(event EventTick
  (params (DeltaSeconds :type Float%20%28single-precision%29)))

(fn ConstructionScript)