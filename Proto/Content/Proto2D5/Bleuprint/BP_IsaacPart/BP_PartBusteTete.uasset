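; BP_PartBusteTete is a bust-and-head body part, apparently for Isaac, that records which arm parts touch it.
; Left and right arm overlap components cast the other actor to a Part or Full arm Blueprint for that side.
; A match stores the corresponding Isaac, pincer or piston sprite in BrasGSPR or BrasDSPR and prints its name, without applying it here.
; The DesTruite event destroys the actor.
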(event OnComponentBeginOverlap(BrasGauche)
  (params (OverlappedComponent :type Primitive%20Component%20Object%20Reference) (OtherActor :type Actor%20Object%20Reference) (OtherComp :type Primitive%20Component%20Object%20Reference) (OtherBodyIndex :type Integer) (bFromSweep :type Boolean) (SweepResult :type Hit%20Result%20Structure%20%28by%20ref%29))
  (Utilities|Casting|CastToBP_PartBrasG OtherActor
    (:then
      (bind _output_get (Variables|Default|SetBrasGSPR "/Game/Proto2D5/Test_Tori/Fixed_Sprite/Isaac/Membres_Gauche/G_Bras_Isaac_Redim_Sprite_2.G_Bras_Isaac_Redim_Sprite_2"))
      (Development|PrintString (Utilities|GetDisplayName _output_get) true true "(R=0.026579,G=0.000000,B=1.000000,A=1.000000)" 5e+01))
    (:CastFailed
      (Utilities|Casting|CastToBP_FullBrasGauche OtherActor)
      (bind _output_get_2 (Variables|Default|SetBrasGSPR "/Game/Proto2D5/Test_Tori/Fixed_Sprite/Isaac/Membres_Gauche/G_Bras_Pince_Redim_Sprite.G_Bras_Pince_Redim_Sprite"))
      (Development|PrintString (Utilities|GetDisplayName _output_get_2) true true "(R=0.026579,G=0.000000,B=1.000000,A=1.000000)" 5e+01))))

(event OnComponentBeginOverlap(BrasDroit)
  (params (OverlappedComponent :type Primitive%20Component%20Object%20Reference) (OtherActor :type Actor%20Object%20Reference) (OtherComp :type Primitive%20Component%20Object%20Reference) (OtherBodyIndex :type Integer) (bFromSweep :type Boolean) (SweepResult :type Hit%20Result%20Structure%20%28by%20ref%29))
  (Utilities|Casting|CastToBP_PartBrasD OtherActor
    (:then
      (bind _output_get (Variables|Default|SetBrasDSPR "/Game/Proto2D5/Test_Tori/Fixed_Sprite/Isaac/Membres_Droit/D_Bras_Isaac_Redim_Sprite_1.D_Bras_Isaac_Redim_Sprite_1"))
      (Development|PrintString (Utilities|GetDisplayName _output_get) true true "(R=1.000000,G=0.000000,B=0.099330,A=1.000000)" 5e+01))
    (:CastFailed
      (Utilities|Casting|CastToBP_FullBrasDroit OtherActor)
      (bind _output_get_2 (Variables|Default|SetBrasDSPR "/Game/Proto2D5/Test_Tori/Fixed_Sprite/Isaac/Membres_Droit/D_Bras_piston_v2_Redim_Sprite.D_Bras_piston_v2_Redim_Sprite"))
      (Development|PrintString (Utilities|GetDisplayName _output_get_2) true true "(R=1.000000,G=0.000000,B=0.099330,A=1.000000)" 5e+01))))

(event Custom|DesTruite
  (Actor|DestroyActor))

(fn ConstructionScript)