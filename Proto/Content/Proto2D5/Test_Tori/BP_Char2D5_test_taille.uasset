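; Test 2.5D player character with axis movement, an overlap-fed inventory widget, searchable spots (E) and an Isaac companion it can call over (A).
; F toggles a part-editing mode that swaps Isaac for separate body-part actors and blends the camera to the torso, then respawns Isaac using the torso's stored sprites.
; In that mode, left mouse drags tagged components through a cursor trace, PhysicsHandle and Tick positioning locked to Isaac's depth.
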(event OnComponentBeginOverlap(CapsuleComponent)
  (params (OverlappedComponent :type Primitive%20Component%20Object%20Reference) (OtherActor :type Actor%20Object%20Reference) (OtherComp :type Primitive%20Component%20Object%20Reference) (OtherBodyIndex :type Integer) (bFromSweep :type Boolean) (SweepResult :type Hit%20Result%20Structure%20%28by%20ref%29))
  ;[0.05628 0.1302 0] Ramassage de l'objet à la collision & affichage dans l'inverterre sur l'écran
  (bind _asbp_object (Utilities|Casting|CastToBP_Object OtherActor))
  (if (Variables|/Game/Proto2D5/Bleuprint/BP_Object.BP_Object_C|GetCanBeDestroyed _asbp_object)
    (if (Variables|Default|GetFirstItem)
      (Variables|Default|SetFirstItem false)
      (else
        (Class|PanelWidget|RemoveChildat (Variables|/Game/Proto2D5/Interface/WBP_Inventary.WBP_Inventary_C|GetVerticalBox_79 (Variables|Default|GetInventory)))))
    (bind _returnvalue (UserInterface|CreateWidget "/Game/Proto2D5/Interface/WBP_Item.WBP_Item_C" 0 (Utilities|Text|ToText(String) (Variables|/Game/Proto2D5/Bleuprint/BP_Object.BP_Object_C|GetItemName _asbp_object)) (Variables|/Game/Proto2D5/Bleuprint/BP_Object.BP_Object_C|GetSpriteInventary _asbp_object)))
    (Class|VerticalBox|AddChildtoVerticalBox (Variables|/Game/Proto2D5/Interface/WBP_Inventary.WBP_Inventary_C|GetVerticalBox_79 (Variables|Default|GetInventory)) _returnvalue)))

(event EventTick
  (params (DeltaSeconds :type Float%20%28single-precision%29))
  (bind _returnvalue (Game|GetPlayerController 0))
  (bind _distancegrabobjet (Variables|Default|GetDistanceGrabObjet))
  (bind (_worldlocation _worlddirection) (Game|Player|ConvertMouseLocationToWorldSpace _returnvalue))
  (bind _returnvalue_2 (* _worlddirection _distancegrabobjet))
  (bind _returnvalue_3 (+ _worldlocation _returnvalue_2))
  (Development|PrintString (Utilities|String|ToString(Vector) (Transformation|GetWorldLocation (Variables|Default|GetSpringArm))) true true "(R=0.000000,G=0.660000,B=1.000000,A=1.000000)" 0.05)
  (if (Variables|Default|GetIsGrabing)
    (Transformation|SetWorldLocation (Variables|Default|GetHit%20Component) (Math|Vector|MakeVector (.x _returnvalue_3) (.y (Variables|Default|GetIsaacWorldLocation)) (.z _returnvalue_3)) false false)))

(event EventBeginPlay
  ;[0 0 0] Add inventary Widget
  (bind _returnvalue (UserInterface|CreateWidget "/Game/Proto2D5/Interface/WBP_Inventary.WBP_Inventary_C"))
  (bind _output_get (Variables|Default|SetInventory _returnvalue))
  (UserInterface|Viewport|AddtoViewport _output_get 0))

(event Input|AxisEvents|InputAxisForward2D5
  (params (AxisValue :type Float%20%28single-precision%29))
  ;[0 0 0] Move left/right
  (if (not (Variables|Default|GetInteractingIsaac))
    (Pawn|Input|AddMovementInput "1.000000,0.000000,0.000000" AxisValue false)
    (if (== AxisValue -2.0)
      (Transformation|SetWorldRotation (Variables|Default|GetSprite) "0.000000,-180.000000,-0.000000" false false)
      (elif (== AxisValue 2.0)
        (Transformation|SetWorldRotation (Variables|Default|GetSprite) "0, 0, 0" false false)))))

(event Input|AxisEvents|InputAxisBack2D5
  (params (AxisValue :type Float%20%28single-precision%29))
  ;[0 0 0] Move forward/back
  (if (not (Variables|Default|GetInteractingIsaac))
    (Pawn|Input|AddMovementInput "0.000000,1.000000,0.000000" AxisValue false)))

(event Input|KeyboardEvents|E
  (params (Key :type Key%20Structure))
  ;[0 0 0] Interact with "BP_Fouille"
  (:Pressed
    (if (Variables|Default|GetIsTriggerFouille)
      (Default|FOUILLE (Variables|Default|GetFouilleBP)))))

(event Input|KeyboardEvents|F
  (params (Key :type Key%20Structure))
  (:Pressed
    (if (or (Variables|Default|GetIsInteractableIsaac) (Variables|Default|GetInteractingIsaac))
      (Utilities|ShowCursor
        (:Out
          (if (Variables|Default|GetInteractingIsaac)
            (bind _returnvalue (Game|SpawnActorfromClass "/Game/Proto2D5/Bleuprint/BP_Isaac1.BP_Isaac1_C" (Math|Conversions|ToTransform(Vector) (Variables|Default|GetIsaacWorldLocation)) "Undefined" "MultiplyWithRoot" 0 0))
            (Variables|Default|SetIsaacBP _returnvalue)
            (Rendering|Components|Sprite|SetSprite (Variables|/Game/Proto2D5/Bleuprint/BP_Isaac1.BP_Isaac1_C|GetBras%20Gauche (Variables|Default|GetIsaacBP)) (Variables|/Game/Proto2D5/Bleuprint/BP_IsaacPart/BP_PartBusteTete.BP_PartBusteTete_C|GetBrasGSPR (Variables|Default|GetNewBuste)))
            (Rendering|Components|Sprite|SetSprite (Variables|/Game/Proto2D5/Bleuprint/BP_Isaac1.BP_Isaac1_C|GetBras%20Droit (Variables|Default|GetIsaacBP)) (Variables|/Game/Proto2D5/Bleuprint/BP_IsaacPart/BP_PartBusteTete.BP_PartBusteTete_C|GetBrasDSPR (Variables|Default|GetNewBuste)))
            (Rendering|Components|Sprite|SetSprite (Variables|/Game/Proto2D5/Bleuprint/BP_Isaac1.BP_Isaac1_C|GetJambe%20Gauche (Variables|Default|GetIsaacBP)) (Variables|/Game/Proto2D5/Bleuprint/BP_IsaacPart/BP_PartBusteTete.BP_PartBusteTete_C|GetJambeGSPR (Variables|Default|GetNewBuste)))
            (Rendering|Components|Sprite|SetSprite (Variables|/Game/Proto2D5/Bleuprint/BP_Isaac1.BP_Isaac1_C|GetJambe%20Droite (Variables|Default|GetIsaacBP)) (Variables|/Game/Proto2D5/Bleuprint/BP_IsaacPart/BP_PartBusteTete.BP_PartBusteTete_C|GetJambeDSPR (Variables|Default|GetNewBuste)))
            (Default|DesTruite (Variables|Default|GetNewBrasG))
            (Default|DesTruite (Variables|Default|GetNewBrasD))
            (Default|DesTruite (Variables|Default|GetNewJambeD))
            (Game|Player|SetViewTargetwithBlend (Game|GetPlayerController 0) self 1.0 "VTBlend_Linear" 0.0 false)
            (Utilities|FlowControl|Delay 1.0)
            (Default|DesTruite (Variables|Default|GetNewBuste))
            (Actor|DestroyActor (Variables|Default|GetTempObject))
            (Variables|Default|SetInteractingIsaac false)
            (else
              (Variables|Default|SetIsaacWorldLocation (Transformation|GetWorldLocation (Variables|/Game/Proto2D5/Bleuprint/BP_Isaac1.BP_Isaac1_C|GetBigBox (Variables|Default|GetIsaacBP))))
              (Variables|Default|SetInteractingIsaac true)
              (Utilities|PlacementDeL'ouvrier
                (:Out
                  (bind _returnvalue_2 (Game|SpawnActorfromClass (Variables|Inventaire|GetUniqueItemFull) (Math|Conversions|ToTransform(Vector) (+ (Variables|Default|GetIsaacWorldLocation) (Math|Vector|MakeVector -1.5e+02 0.0 (+ 100 (* (stale _array_index) -30))))) "Undefined" "MultiplyWithRoot" 0 0))
                  (Variables|Default|SetTempObject _returnvalue_2)
                  (bind _returnvalue_3 (Game|SpawnActorfromClass "/Game/Proto2D5/Bleuprint/BP_IsaacPart/BP_PartBrasG.BP_PartBrasG_C" (Math|Conversions|ToTransform(Vector) (Transformation|GetWorldLocation (Variables|/Game/Proto2D5/Bleuprint/BP_Isaac1.BP_Isaac1_C|GetBras%20Gauche (Variables|Default|GetIsaacBP)))) "Undefined" "MultiplyWithRoot" 0 0))
                  (bind _output_get (Variables|Default|SetNewBrasG _returnvalue_3))
                  (Rendering|Components|Sprite|SetSprite (Variables|/Game/Proto2D5/Bleuprint/BP_IsaacPart/BP_PartBrasG.BP_PartBrasG_C|GetSprite _output_get) (Sprite|GetSprite (Variables|/Game/Proto2D5/Bleuprint/BP_Isaac1.BP_Isaac1_C|GetJambe%20Gauche (Variables|Default|GetIsaacBP))))
                  (bind _returnvalue_4 (Game|SpawnActorfromClass "/Game/Proto2D5/Bleuprint/BP_IsaacPart/BP_PartBrasD.BP_PartBrasD_C" (Math|Conversions|ToTransform(Vector) (Transformation|GetWorldLocation (Variables|/Game/Proto2D5/Bleuprint/BP_Isaac1.BP_Isaac1_C|GetBras%20Droit (Variables|Default|GetIsaacBP)))) "Undefined" "MultiplyWithRoot" 0 0))
                  (bind _output_get_2 (Variables|Default|SetNewBrasD _returnvalue_4))
                  (Rendering|Components|Sprite|SetSprite (Variables|/Game/Proto2D5/Bleuprint/BP_IsaacPart/BP_PartBrasD.BP_PartBrasD_C|GetSprite _output_get_2) (Sprite|GetSprite (Variables|/Game/Proto2D5/Bleuprint/BP_Isaac1.BP_Isaac1_C|GetBras%20Droit (Variables|Default|GetIsaacBP))))
                  (bind _returnvalue_5 (Game|SpawnActorfromClass "/Game/Proto2D5/Bleuprint/BP_IsaacPart/BP_PartJambeD.BP_PartJambeD_C" (Math|Conversions|ToTransform(Vector) (Transformation|GetWorldLocation (Variables|/Game/Proto2D5/Bleuprint/BP_Isaac1.BP_Isaac1_C|GetJambe%20Droite (Variables|Default|GetIsaacBP)))) "Undefined" "MultiplyWithRoot" 0 0))
                  (bind _output_get_3 (Variables|Default|SetNewJambeD _returnvalue_5))
                  (Rendering|Components|Sprite|SetSprite (Variables|/Game/Proto2D5/Bleuprint/BP_IsaacPart/BP_PartJambeD.BP_PartJambeD_C|GetSprite _output_get_3) (Sprite|GetSprite (Variables|/Game/Proto2D5/Bleuprint/BP_Isaac1.BP_Isaac1_C|GetJambe%20Droite (Variables|Default|GetIsaacBP))))
                  (Rendering|Components|Sprite|SetSprite (Variables|/Game/Proto2D5/Bleuprint/BP_IsaacPart/BP_PartJambeD.BP_PartJambeD_C|GetJambe%20Gauche _output_get_3) (Sprite|GetSprite (Variables|/Game/Proto2D5/Bleuprint/BP_Isaac1.BP_Isaac1_C|GetJambe%20Gauche (Variables|Default|GetIsaacBP))))
                  (bind _returnvalue_6 (Game|SpawnActorfromClass "/Game/Proto2D5/Bleuprint/BP_IsaacPart/BP_PartBusteTete.BP_PartBusteTete_C" (Math|Conversions|ToTransform(Vector) (Transformation|GetWorldLocation (Variables|/Game/Proto2D5/Bleuprint/BP_Isaac1.BP_Isaac1_C|GetBuste (Variables|Default|GetIsaacBP)))) "Undefined" "MultiplyWithRoot" 0 0))
                  (bind _output_get_4 (Variables|Default|SetNewBuste _returnvalue_6))
                  (Game|Player|SetViewTargetwithBlend (Game|GetPlayerController 0) _output_get_4 1.0 "VTBlend_Linear" 0.0 false)
                  (Default|Disparition (Variables|Default|GetIsaacBP)))))))))))

(event Input|MouseEvents|LeftMouseButton
  (params (Key :type Key%20Structure))
  ;[0.1023 0.4427 0] Grip
  (:Pressed
    (if (Variables|Default|GetInteractingIsaac)
      (Utilities|GrabComponent
        (:Out
          (Variables|Default|SetIsGrabing true)))))
  (:Released
    (if (Variables|Default|GetInteractingIsaac)
      (Variables|Default|SetHit%20Component 0)
      (Physics|Components|PhysicsHandle|ReleaseComponent (Variables|Default|GetPhysicsHandle))
      (Variables|Default|SetIsGrabing false))))

(event Input|KeyboardEvents|A
  (params (Key :type Key%20Structure))
  (:Pressed
    (Default|MoveToo (Variables|Default|GetIsaacBP) (Transformation|GetActorLocation))))

(fn ConstructionScript)